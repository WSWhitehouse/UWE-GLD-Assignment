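; Villager interactable that shows configurable text when used and can set the player's objective.
; Interact reveals the text component, and Tick counts up to TextVisibleAmount before hiding it again, with interaction disabled while it shows.
; If AdvanceObjective is on and ObjectiveAdvanced is false, it calls SetObjective on the first ThirdPersonCharacter found; this graph never sets ObjectiveAdvanced.
; Getters supply hover text and name, and opt out of inventory pickup.
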(event EventBeginPlay
  (Rendering|Components|TextRender|SetText (Variables|Default|GetTextComponent) (Variables|Default|GetText))
  (Rendering|SetVisibility (Variables|Default|GetTextComponent) false true))

(event EventTick
  (params (DeltaSeconds :type Float%20%28single-precision%29))
  (if (Variables|Default|GetTextVisable)
    (if (>= (Variables|Default|GetTimer) (Variables|Default|GetTextVisibleAmount))
      (Variables|Default|SetTimer 0.0)
      (Variables|Default|SetTextVisable false)
      (Rendering|SetVisibility (Variables|Default|GetTextComponent) false true)
      (else
        (Variables|Default|SetTimer (+ DeltaSeconds (Variables|Default|GetTimer)))))))

(event EventInteract
  (Variables|Default|SetTextVisable true)
  (Rendering|SetVisibility (Variables|Default|GetTextComponent) true true)
  (if (Variables|Default|GetAdvanceObjective)
    (if (not (Variables|Default|GetObjectiveAdvanced))
      (bind _outactors (Actor|GetAllActorsOfClass "/Game/CharacterController/Blueprints/ThirdPersonCharacter.ThirdPersonCharacter_C"))
      (Default|SetObjective (Utilities|Array|Get(acopy) _outactors) (Variables|Default|GetObjectiveToAdvanceTo)))))

(fn ConstructionScript
  (Rendering|Components|TextRender|SetText (Variables|Default|GetTextComponent) (Variables|Default|GetText)))

(fn GetAddtoInventory
  (return false))

(fn GetHoverText
  (return (Utilities|String|ToString(Text) (Variables|Default|GetHoverText))))

(fn GetImage
  (return 0))

(fn GetIsInteractable
  (return (not (Variables|Default|GetTextVisable))))

(fn GetName
  (return "villager"))