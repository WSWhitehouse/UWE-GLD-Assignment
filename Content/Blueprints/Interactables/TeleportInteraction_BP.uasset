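; Interactable actor that teleports the player character to a preset transform when used.
; On BeginPlay it caches the first ThirdPersonCharacter found in the level, and Interact teleports that character to the location and rotation of TeleportTransform.
; Its getter functions mark it as always interactable and never added to inventory, supplying hover text but no name or image.
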(event EventBeginPlay
  (bind _outactors (Actor|GetAllActorsOfClass "/Game/CharacterController/Blueprints/ThirdPersonCharacter.ThirdPersonCharacter_C"))
  (Variables|Default|SetCharacterController (Utilities|Array|Get(acopy) _outactors)))

(event Collision|EventActorBeginOverlap
  (params (OtherActor :type Actor%20Object%20Reference)))

(event EventTick
  (params (DeltaSeconds :type Float%20%28single-precision%29)))

(event EventInteract
  (bind _teleporttransform (Variables|Default|GetTeleportTransform))
  (bind (_location _rotation) (Math|Transform|BreakTransform _teleporttransform))
  (Transformation|Teleport (Variables|Default|GetCharacterController) _location _rotation))

(fn ConstructionScript)

(fn GetAddtoInventory
  (return false))

(fn GetHoverText
  (return (Utilities|String|ToString(Text) (Variables|Default|GetHoverText))))

(fn GetImage
  (return 0))

(fn GetIsInteractable
  (return true))

(fn GetName
  (return ""))