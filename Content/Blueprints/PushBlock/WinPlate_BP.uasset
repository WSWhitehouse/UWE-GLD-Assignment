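; WinPlate_BP is a goal plate for push blocks that tracks whether a target block is resting on it.
; On BeginPlay it gives its plane a glowing red dynamic material instance.
; Box overlaps with the cube of a PushBlock_BP flagged as Target turn the plate green and set WinPlateActive.
; When that cube leaves, the plate reverts to red and clears the flag.
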(event OnComponentBeginOverlap(Box)
  (params (OverlappedComponent :type Primitive%20Component%20Object%20Reference) (OtherActor :type Actor%20Object%20Reference) (OtherComp :type Primitive%20Component%20Object%20Reference) (OtherBodyIndex :type Integer) (bFromSweep :type Boolean) (SweepResult :type Hit%20Result%20Structure%20%28by%20ref%29))
  (bind _aspush_block_bp (Utilities|Casting|CastToPushBlock_BP OtherActor))
  (if (== (Variables|/Game/Blueprints/PushBlock/PushBlock_BP.PushBlock_BP_C|GetCube _aspush_block_bp) OtherComp)
    (if (Variables|/Game/Blueprints/PushBlock/PushBlock_BP.PushBlock_BP_C|GetTarget? _aspush_block_bp)
      (Rendering|Material|SetVectorParameterValue (stale EventBeginPlay _returnvalue) "Colour" "(R=0.000000,G=1.000000,B=0.000000,A=1.000000)" :!class /Script/Engine.MaterialInstanceDynamic)
      (Variables|Default|SetWinPlateActive true))))

(event OnComponentEndOverlap(Box)
  (params (OverlappedComponent :type Primitive%20Component%20Object%20Reference) (OtherActor :type Actor%20Object%20Reference) (OtherComp :type Primitive%20Component%20Object%20Reference) (OtherBodyIndex :type Integer))
  (bind _aspush_block_bp (Utilities|Casting|CastToPushBlock_BP OtherActor))
  (if (== (Variables|/Game/Blueprints/PushBlock/PushBlock_BP.PushBlock_BP_C|GetCube _aspush_block_bp) OtherComp)
    (if (Variables|/Game/Blueprints/PushBlock/PushBlock_BP.PushBlock_BP_C|GetTarget? _aspush_block_bp)
      (Rendering|Material|SetVectorParameterValue (stale EventBeginPlay _returnvalue) "Colour" "(R=1.000000,G=0.000000,B=0.000000,A=1.000000)" :!class /Script/Engine.MaterialInstanceDynamic)
      (Variables|Default|SetWinPlateActive false))))

(event EventBeginPlay
  (bind _plane (Variables|Default|GetPlane))
  (bind _returnvalue (Rendering|Material|CreateDynamicMaterialInstance _plane 0 "/Game/Materials/DefaultRed_M.DefaultRed_M" "None" :!class /Script/Engine.PrimitiveComponent))
  (Rendering|Material|SetMaterial _plane 0 _returnvalue)
  (Rendering|Material|SetScalarParameterValue _returnvalue "Intensity" 2e+01 :!class /Script/Engine.MaterialInstanceDynamic)
  (Rendering|Material|SetVectorParameterValue _returnvalue "Colour" "(R=1.000000,G=0.000000,B=0.000000,A=1.000000)" :!class /Script/Engine.MaterialInstanceDynamic))

(fn ConstructionScript)