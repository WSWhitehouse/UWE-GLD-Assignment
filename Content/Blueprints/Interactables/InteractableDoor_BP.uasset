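; An interactable door Blueprint that the player opens when carrying a key or crowbar.
; On BeginPlay it caches the first ThirdPersonCharacter; Interact scans that character's inventory item names for a match.
; Opening works by enabling physics simulation on the Door component, which also makes it report as no longer interactable.
; Interface-style getters supply the hover prompt and keep the door out of the inventory.
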(event EventBeginPlay
  (bind _outactors (Actor|GetAllActorsOfClass "/Game/CharacterController/Blueprints/ThirdPersonCharacter.ThirdPersonCharacter_C"))
  (Variables|Default|SetCharacterController (Utilities|Array|Get(acopy) _outactors)))

(event Collision|EventActorBeginOverlap
  (params (OtherActor :type Actor%20Object%20Reference)))

(event EventTick
  (params (DeltaSeconds :type Float%20%28single-precision%29)))

(event EventInteract
  (bind _charactercontroller (Variables|Default|GetCharacterController))
  (bind _inventory (Variables|/Game/CharacterController/Blueprints/ThirdPersonCharacter.ThirdPersonCharacter_C|GetInventory _charactercontroller))
  (bind _index (Utilities|FlowControl|ForLoopwithBreak 0 (Utilities|Array|Length _inventory))
    (:LoopBody
      (bind _name (Class|InteractableIBP|GetName(Message) (Utilities|Array|Get(acopy) _inventory _index)))
      (if (or (Utilities|Enum|Equal(Enum) _name "Key") (Utilities|Enum|Equal(Enum) _name "Crowbar"))
        (Physics|SetSimulatePhysics (Variables|Default|GetDoor) true)))))

(fn ConstructionScript)

(fn GetAddtoInventory
  (return false))

(fn GetHoverText
  (return "Open Door (Requires Key)"))

(fn GetImage
  (return 0))

(fn GetIsInteractable
  (return (not (Physics|IsSimulatingPhysics (Variables|Default|GetDoor) "None"))))

(fn GetName
  (return ""))