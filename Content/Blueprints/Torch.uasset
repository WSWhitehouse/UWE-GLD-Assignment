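; Torch actor with a fire particle effect and a light that flickers at random.
; Each Tick, with a chance set by ChangeLightPercentage, it gives the light a random intensity from LightIntensity and a random source radius from LightRange.
; EnableTorch and DisableTorch show or hide both the fire particles and the light, while the flicker logic on Tick runs regardless of that state.
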(event EventBeginPlay)

(event Collision|EventActorBeginOverlap
  (params (OtherActor :type Actor%20Object%20Reference)))

(event EventTick
  (params (DeltaSeconds :type Float%20%28single-precision%29))
  (bind _light (Variables|Default|GetLight))
  (bind _lightintensity (Variables|Default|GetLightIntensity))
  (bind _lightrange (Variables|Default|GetLightRange))
  (bind (_lowerbound _upperbound) (Utilities|Struct|BreakFloatRange _lightrange))
  (bind (_lowerbound_2 _upperbound_2) (Utilities|Struct|BreakFloatRange _lightintensity))
  (if (< (Math|Random|RandomFloat) (Variables|Default|GetChangeLightPercentage))
    (Rendering|Components|Light|SetIntensity _light (Math|Random|RandomFloatinRange (.Value (Utilities|Struct|BreakFloatRangeBound _lowerbound_2)) (.Value (Utilities|Struct|BreakFloatRangeBound _upperbound_2))))
    (Class|PointLightComponent|SetSourceRadius _light (Math|Random|RandomFloatinRange (.Value (Utilities|Struct|BreakFloatRangeBound _lowerbound)) (.Value (Utilities|Struct|BreakFloatRangeBound _upperbound))))))

(fn ConstructionScript)

(fn EnableTorch
  (Rendering|SetVisibility (Variables|Default|GetFire_PS) true false)
  (Rendering|SetVisibility (Variables|Default|GetLight) true false))

(fn DisableTorch
  (Rendering|SetVisibility (Variables|Default|GetFire_PS) false false)
  (Rendering|SetVisibility (Variables|Default|GetLight) false false))