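; Interactable crowbar pickup that the player can add to their inventory.
; It supplies the hover prompt and item name, always reports as interactable, and returns an empty image.
; Adding it to inventory returns true and, rather than destroying the actor, moves it to the world origin at zero scale to hide it.
; The event graph and construction script have no logic.
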(event EventBeginPlay)

(event Collision|EventActorBeginOverlap
  (params (OtherActor :type Actor%20Object%20Reference)))

(event EventTick
  (params (DeltaSeconds :type Float%20%28single-precision%29)))

(fn ConstructionScript)

(fn GetAddtoInventory
  (Transformation|SetActorTransform (Math|Transform|MakeTransform "0, 0, 0" "0, 0, 0" "0.000000,0.000000,0.000000"))
  (return true))

(fn GetHoverText
  (return "Pick up Crowbar"))

(fn GetImage
  (return 0))

(fn GetIsInteractable
  (return true))

(fn GetName
  (return "Crowbar"))