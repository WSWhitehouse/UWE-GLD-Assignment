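; One-shot portal actor that teleports the third-person character to the SpawnTransform location and rotation, and halves that character's gravity scale.
; A hit on the Portal component triggers it only while PortalActive is set and EnteredPortal is still false.
; On entry it calls PortalEntered, hides the portal and its children, disables the portal's collision and plays a 2D sound.
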(event OnComponentHit(Portal)
  (params (HitComponent :type Primitive%20Component%20Object%20Reference) (OtherActor :type Actor%20Object%20Reference) (OtherComp :type Primitive%20Component%20Object%20Reference) (NormalImpulse :type Vector :default "0, 0, 0") (Hit :type Hit%20Result%20Structure%20%28by%20ref%29))
  (bind _spawntransform (Variables|Default|GetSpawnTransform))
  (bind _portal (Variables|Default|GetPortal))
  (bind _returnvalue (Transformation|GetWorldTransform _spawntransform))
  (bind (_location _rotation) (Math|Transform|BreakTransform _returnvalue))
  (if (and (Variables|Default|GetPortalActive) (not (Variables|Default|GetEnteredPortal)))
    (bind _asthird_person_character (Utilities|Casting|CastToThirdPersonCharacter OtherActor))
    (Variables|Default|SetEnteredPortal true)
    (Transformation|Teleport _asthird_person_character _location _rotation)
    (Variables|/Script/Engine.CharacterMovementComponent|SetGravityScale (Variables|/Script/Engine.Character|GetCharacterMovement _asthird_person_character) (/ (Variables|/Script/Engine.CharacterMovementComponent|GetGravityScale (Variables|/Script/Engine.Character|GetCharacterMovement _asthird_person_character)) 2.0))
    (Default|CallPortalEntered)
    (Rendering|SetVisibility _portal false true)
    (Collision|SetCollisionEnabled _portal "NoCollision")
    (Audio|PlaySound2D "/Game/Audio/PortalSound.PortalSound" 1.0 1.0 0.0 0 0)))

(event EventBeginPlay)

(event Collision|EventActorBeginOverlap
  (params (OtherActor :type Actor%20Object%20Reference)))

(event EventTick
  (params (DeltaSeconds :type Float%20%28single-precision%29)))

(fn ConstructionScript)