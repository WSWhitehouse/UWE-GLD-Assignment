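; GameManager is an actor Blueprint that drives a timed change of the game's Objectives state.
; On Tick it adds delta time to Timer while Objectives holds one specific enum value.
; A second sequence branch sets Objectives to another value whenever Timer has reached MaxTime, regardless of the current objective.
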(event EventBeginPlay)

(event Collision|EventActorBeginOverlap
  (params (OtherActor :type Actor%20Object%20Reference)))

(event EventTick
  (params (DeltaSeconds :type Float%20%28single-precision%29))
  (Utilities|FlowControl|Sequence
    (:then_0
      (if (Utilities|Enum|Equal(Enum) (Variables|Default|GetObjectives) "NewEnumerator6")
        (Variables|Default|SetTimer (+ DeltaSeconds (Variables|Default|GetTimer)))))
    (:then_1
      (if (>= (Variables|Default|GetTimer) (Variables|Default|GetMaxTime))
        (Variables|Default|SetObjectives "NewEnumerator8")))))

(fn ConstructionScript)