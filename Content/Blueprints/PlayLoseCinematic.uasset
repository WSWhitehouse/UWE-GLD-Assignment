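; Actor that plays the lose cinematic when the game is lost, then ends the game.
; It hides the Monster, Player and Ground actors, with their child components, on BeginPlay.
; PlayCinematic reveals them, starts the LoseCinematic level sequence and binds an event to its finish.
; A Quit function, presumably that finish callback, closes the game.
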(event EventBeginPlay
  (Rendering|SetVisibility (Variables|/Script/Engine.Actor|GetRootComponent (Variables|Default|GetMonster)) false true)
  (Rendering|SetVisibility (Variables|/Script/Engine.Actor|GetRootComponent (Variables|Default|GetPlayer)) false true)
  (Rendering|SetVisibility (Variables|/Script/Engine.Actor|GetRootComponent (Variables|Default|GetGround)) false true))

(fn ConstructionScript)

(fn PlayCinematic
  (bind _losecinematic (Variables|Default|GetLoseCinematic))
  (bind _sequenceplayer (Variables|/Script/LevelSequence.LevelSequenceActor|GetSequencePlayer _losecinematic))
  (Rendering|SetVisibility (Variables|/Script/Engine.Actor|GetRootComponent (Variables|Default|GetMonster)) true true)
  (Rendering|SetVisibility (Variables|/Script/Engine.Actor|GetRootComponent (Variables|Default|GetPlayer)) true true)
  (Rendering|SetVisibility (Variables|/Script/Engine.Actor|GetRootComponent (Variables|Default|GetGround)) true true)
  (Sequencer|Player|Play _sequenceplayer :!class /Script/MovieScene.MovieSceneSequencePlayer)
  (EventDispatchers|BindEventtoOnFinished _sequenceplayer (EventDispatchers|CreateEvent :!event Quit)))

(fn Quit
  (Game|QuitGame 0 "Quit" false))