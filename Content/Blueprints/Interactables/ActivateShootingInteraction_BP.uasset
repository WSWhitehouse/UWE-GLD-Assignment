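; An interactable "Strange Artefact" that unlocks the Dark Energy shooting ability.
; The unlock runs inside GetAddToInventory, which calls ShootingEnabled, shows a popup through the first ThirdPersonCharacter's MainUI, and returns true.
; Instead of being destroyed, the actor is moved to the origin at zero scale.
; The other getters supply name and hover text; GetImage returns nothing and the Interact event is empty.
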(event EventBeginPlay)

(event Collision|EventActorBeginOverlap
  (params (OtherActor :type Actor%20Object%20Reference)))

(event EventTick
  (params (DeltaSeconds :type Float%20%28single-precision%29)))

(event EventInteract)

(fn ConstructionScript)

(fn GetAddtoInventory
  (Transformation|SetActorTransform (Math|Transform|MakeTransform "0, 0, 0" "0, 0, 0" "0.000000,0.000000,0.000000"))
  (Default|CallShootingEnabled)
  (bind _outactors (Actor|GetAllActorsOfClass "/Game/CharacterController/Blueprints/ThirdPersonCharacter.ThirdPersonCharacter_C"))
  (Default|ShowPopupText (Variables|/Game/CharacterController/Blueprints/ThirdPersonCharacter.ThirdPersonCharacter_C|GetMainUI (Utilities|Array|Get(acopy) _outactors)) 5.0 "Dark Energy Ability Unlocked! 
Use Left Click to fire!")
  (return true))

(fn GetHoverText
  (return "Touch Strange Artefact"))

(fn GetImage
  (return 0))

(fn GetIsInteractable
  (return true))

(fn GetName
  (return "Dark Energy"))