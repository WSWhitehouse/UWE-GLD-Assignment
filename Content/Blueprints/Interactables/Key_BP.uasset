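; Key pickup actor that the player can hover over and add to an inventory as "Key".
; Interaction getters supply the hover text, name, inventory image and an always-interactable flag.
; GetAddToInventory returns true after moving the actor to the world origin at zero scale, hiding it rather than destroying it.
; The Interact event and construction script are empty.
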(event EventBeginPlay)

(event Collision|EventActorBeginOverlap
  (params (OtherActor :type Actor%20Object%20Reference)))

(event EventTick
  (params (DeltaSeconds :type Float%20%28single-precision%29)))

(event EventInteract)

(fn ConstructionScript)

(fn GetAddtoInventory
  (Transformation|SetActorTransform (Math|Transform|MakeTransform "0, 0, 0" "0, 0, 0" "0.000000,0.000000,0.000000"))
  (return true))

(fn GetHoverText
  (return "Pick up Key"))

(fn GetImage
  (return (Variables|Default|GetInvImage)))

(fn GetIsInteractable
  (return true))

(fn GetName
  (return "Key"))