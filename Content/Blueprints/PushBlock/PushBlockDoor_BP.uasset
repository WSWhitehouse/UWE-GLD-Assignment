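; Push-block puzzle door that opens permanently once its referenced WinPlate becomes active.
; BeginPlay gives the mesh a dynamic material instance with a red, glowing-intensity setup.
; Tick polls the plate until the door opens, then sets the material green, disables collision, plays a 2D sound and hides the mesh.
; A DoorOpened flag makes the opening happen only once, with no path to close again.
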(event Collision|EventActorBeginOverlap
  (params (OtherActor :type Actor%20Object%20Reference)))

(event EventTick
  (params (DeltaSeconds :type Float%20%28single-precision%29))
  (bind _staticmesh (Variables|Default|GetStaticMesh))
  (if (not (Variables|Default|GetDoorOpened))
    (if (Variables|/Game/Blueprints/PushBlock/WinPlate_BP.WinPlate_BP_C|GetWinPlateActive (Variables|Default|GetWinPlate))
      (Rendering|Material|SetVectorParameterValue (Variables|Default|GetMaterial) "Colour" "(R=0.000000,G=1.000000,B=0.000000,A=0.200000)" :!class /Script/Engine.MaterialInstanceDynamic)
      (Collision|SetCollisionEnabled _staticmesh "NoCollision")
      (Audio|PlaySound2D (Variables|Default|GetSound) 1.0 1.0 0.0 0 0)
      (Variables|Default|SetDoorOpened true)
      (Rendering|SetVisibility _staticmesh false false))))

(event EventBeginPlay
  (bind _staticmesh (Variables|Default|GetStaticMesh))
  (bind _returnvalue (Rendering|Material|CreateDynamicMaterialInstance _staticmesh 0 "/Game/Materials/DefaultRed_M.DefaultRed_M" "None" :!class /Script/Engine.PrimitiveComponent))
  (bind _output_get (Variables|Default|SetMaterial _returnvalue))
  (Rendering|Material|SetMaterial _staticmesh 0 _output_get)
  (Rendering|Material|SetScalarParameterValue _output_get "Intensity" 2e+01 :!class /Script/Engine.MaterialInstanceDynamic)
  (Rendering|Material|SetVectorParameterValue _output_get "Colour" "(R=1.000000,G=0.000000,B=0.000000,A=1.000000)" :!class /Script/Engine.MaterialInstanceDynamic))

(fn ConstructionScript)