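; PushBlock_BP is a pushable cube that the ThirdPersonCharacter can shove around.
; Two trigger volumes, XBox and YBox, set the character's IsPushing flag and turn on the cube's physics simulation while overlapped, reversing both on exit.
; The construction script gives the cube a dynamic DefaultRed_M instance, colored green when Target is set and red otherwise.
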(event OnComponentBeginOverlap(yBox)
  (params (OverlappedComponent :type Primitive%20Component%20Object%20Reference) (OtherActor :type Actor%20Object%20Reference) (OtherComp :type Primitive%20Component%20Object%20Reference) (OtherBodyIndex :type Integer) (bFromSweep :type Boolean) (SweepResult :type Hit%20Result%20Structure%20%28by%20ref%29))
  (bind _asthird_person_character (Utilities|Casting|CastToThirdPersonCharacter OtherActor))
  (Variables|/Game/CharacterController/Blueprints/ThirdPersonCharacter.ThirdPersonCharacter_C|SetIsPushing _asthird_person_character true)
  (Physics|SetSimulatePhysics (Variables|Default|GetCube) true))

(event OnComponentEndOverlap(yBox)
  (params (OverlappedComponent :type Primitive%20Component%20Object%20Reference) (OtherActor :type Actor%20Object%20Reference) (OtherComp :type Primitive%20Component%20Object%20Reference) (OtherBodyIndex :type Integer))
  (bind _asthird_person_character (Utilities|Casting|CastToThirdPersonCharacter OtherActor))
  (Variables|/Game/CharacterController/Blueprints/ThirdPersonCharacter.ThirdPersonCharacter_C|SetIsPushing _asthird_person_character false)
  (Physics|SetSimulatePhysics (Variables|Default|GetCube) false))

(event OnComponentBeginOverlap(xBox)
  (params (OverlappedComponent :type Primitive%20Component%20Object%20Reference) (OtherActor :type Actor%20Object%20Reference) (OtherComp :type Primitive%20Component%20Object%20Reference) (OtherBodyIndex :type Integer) (bFromSweep :type Boolean) (SweepResult :type Hit%20Result%20Structure%20%28by%20ref%29))
  (bind _asthird_person_character (Utilities|Casting|CastToThirdPersonCharacter OtherActor))
  (Variables|/Game/CharacterController/Blueprints/ThirdPersonCharacter.ThirdPersonCharacter_C|SetIsPushing _asthird_person_character true)
  (Physics|SetSimulatePhysics (Variables|Default|GetCube) true))

(event OnComponentEndOverlap(xBox)
  (params (OverlappedComponent :type Primitive%20Component%20Object%20Reference) (OtherActor :type Actor%20Object%20Reference) (OtherComp :type Primitive%20Component%20Object%20Reference) (OtherBodyIndex :type Integer))
  (bind _asthird_person_character (Utilities|Casting|CastToThirdPersonCharacter OtherActor))
  (Variables|/Game/CharacterController/Blueprints/ThirdPersonCharacter.ThirdPersonCharacter_C|SetIsPushing _asthird_person_character false)
  (Physics|SetSimulatePhysics (Variables|Default|GetCube) false))

(fn ConstructionScript
  (bind _cube (Variables|Default|GetCube))
  (bind _returnvalue (Rendering|Material|CreateDynamicMaterialInstance _cube 0 "/Game/Materials/DefaultRed_M.DefaultRed_M" "None" :!class /Script/Engine.PrimitiveComponent))
  (Rendering|Material|SetMaterial _cube 0 _returnvalue)
  (if (Variables|Default|GetTarget?)
    (Rendering|Material|SetVectorParameterValue _returnvalue "Colour" "(R=0.000000,G=1.000000,B=0.000000,A=1.000000)" :!class /Script/Engine.MaterialInstanceDynamic)
    (else
      (Rendering|Material|SetVectorParameterValue _returnvalue "Colour" "(R=1.000000,G=0.000000,B=0.000000,A=1.000000)" :!class /Script/Engine.MaterialInstanceDynamic))))