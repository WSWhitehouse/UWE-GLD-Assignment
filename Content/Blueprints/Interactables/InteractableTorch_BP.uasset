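; Interactable torch pickup that can be added to the inventory and toggles a torch on and off.
; On BeginPlay it spawns a separate Torch actor owned by the first ThirdPersonCharacter found in the level.
; Interact enables or disables that Torch based on TorchEnabled.
; Getter functions supply name and hover text, while GetAddToInventory hides the pickup by moving it to the origin at zero scale.
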(event EventBeginPlay
  (|CallParentFunction)
  (bind _outactors (Actor|GetAllActorsOfClass "/Game/CharacterController/Blueprints/ThirdPersonCharacter.ThirdPersonCharacter_C"))
  (bind _output_get (Variables|Default|SetCharacterController (Utilities|Array|Get(acopy) _outactors)))
  (bind _returnvalue (Game|SpawnActorfromClass "/Game/Blueprints/Torch.Torch_C" (Math|Transform|MakeTransform "0, 0, 0") "Undefined" _output_get 0))
  (Variables|Default|SetTorch _returnvalue))

(event Collision|EventActorBeginOverlap
  (params (OtherActor :type Actor%20Object%20Reference))
  (|CallParentFunction OtherActor) ; This node is disabled and will not be called.\nDrag off pins to build functionality.
)

(event EventTick
  (params (DeltaSeconds :type Float%20%28single-precision%29))
  (|CallParentFunction DeltaSeconds) ; This node is disabled and will not be called.\nDrag off pins to build functionality.
)

(event EventInteract
  (bind _torch (Variables|Default|GetTorch))
  (if (Variables|Default|GetTorchEnabled)
    (Default|DisableTorch _torch)
    (else
      (Default|EnableTorch _torch))))

(fn ConstructionScript
  (|CallParentFunction))

(fn GetAddtoInventory
  (Transformation|SetActorTransform (Math|Transform|MakeTransform "0, 0, 0" "0, 0, 0" "0.000000,0.000000,0.000000"))
  (return true))

(fn GetHoverText
  (return "Pick up Torch"))

(fn GetImage
  (return 0))

(fn GetIsInteractable
  (return true))

(fn GetName
  (return "Torch"))