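; WeatherSystem_BP is a weather actor that plays a looping-style ambient weather sound and drives random lightning and thunder.
; On BeginPlay it starts the weather audio, then runs an endless delay-driven loop that waits, flickers LightningLight through a random number of strikes, switches it off and plays a delayed 2D thunder sound.
; Timing, intensity and strike count come from range variables sampled by two random helper functions.
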(event EventBeginPlay
  (bind _audio (Variables|Default|GetAudio))
  (bind _lightninglight (Variables|Default|GetLightningLight))
  (Utilities|FlowControl|Sequence
    (:then_0
      (Audio|Components|Audio|SetSound _audio (Variables|Default|GetWeatherSound))
      (Audio|Components|Audio|Play _audio 0.0))
    (:then_1
      (bind _randomval (CallFunction|GetRandomValueinRangeFloat (Variables|Default|GetDelayBetweenLightning) :!label _label))
      (Utilities|FlowControl|Delay _randomval)
      (bind _randomval_2 (CallFunction|GetRandomValueinRangeInt (Variables|Default|GetNumOfStrikesAtATime)))
      (bind _output_get (Variables|Default|Setindex _randomval_2))
      (if (> _output_get 0) :!label _label_2
        (bind _randomval_3 (CallFunction|GetRandomValueinRangeFloat (Variables|Default|GetLightningIntensity)))
        (Rendering|Components|Light|SetIntensity _lightninglight _randomval_3)
        (bind _randomval_4 (CallFunction|GetRandomValueinRangeFloat (Variables|Default|GetDelayBetweenLightningStrikes)))
        (Utilities|FlowControl|Delay _randomval_4)
        (Variables|Default|Setindex (- (Variables|Default|Getindex) 1))
        (goto _label_2)
        (else
          (Rendering|Components|Light|SetIntensity _lightninglight 0.0)
          (bind _randomval_5 (CallFunction|GetRandomValueinRangeFloat (Variables|Default|GetDelayBetweenLightningSound)))
          (Utilities|FlowControl|Delay _randomval_5)
          (Audio|PlaySound2D (Variables|Default|GetLightningSound) 1.0 1.0 0.0 0 0)
          (goto _label))))))

(fn ConstructionScript)

(fn GetRandomValueinRangeFloat
  (params (Range :type Float%20Range%20Structure))
  (bind (_lowerbound _upperbound) (Utilities|Struct|BreakFloatRange Range))
  (return (Math|Random|RandomFloatinRange (.Value (Utilities|Struct|BreakFloatRangeBound _lowerbound)) (.Value (Utilities|Struct|BreakFloatRangeBound _upperbound)))))

(fn GetRandomValueinRangeInt
  (params (Range :type Int%2032%20Range%20Structure))
  (bind (_lowerbound _upperbound) (Utilities|Struct|BreakInt32Range Range))
  (return (Math|Random|RandomIntegerinRange (.Value (Utilities|Struct|BreakInt32RangeBound _lowerbound)) (.Value (Utilities|Struct|BreakInt32RangeBound _upperbound)))))