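; Blueprint that swaps the level between an Overworld and an Other Side state when the portal is entered.
; On BeginPlay it caches actors by tag, showing and enabling collision on Overworld actors while hiding Other Side ones.
; It binds to the first Portal_BP's entered event, which reverses both groups' visibility and collision.
; The swap is one-way, with no path back to the Overworld state.
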(event Custom|PortalEntered_Event
  (Utilities|FlowControl|Sequence
    (:then_0
      (for _array_element (Variables|Default|GetOtherSideActors)
        (Rendering|SetVisibility (Variables|/Script/Engine.Actor|GetRootComponent _array_element) true true)
        (Collision|SetActorEnableCollision _array_element true)))
    (:then_1
      (for _array_element_2 (Variables|Default|GetOverworldActors)
        (Rendering|SetVisibility (Variables|/Script/Engine.Actor|GetRootComponent _array_element_2) false true)
        (Collision|SetActorEnableCollision _array_element_2 false)))))

(event EventBeginPlay
  (Utilities|FlowControl|Sequence
    (:then_0
      (bind _outactors (Actor|GetAllActorswithTag (Variables|Default|GetOtherSideTag)))
      (bind _output_get (Variables|Default|SetOtherSideActors _outactors))
      (for _array_element _output_get
        (Rendering|SetVisibility (Variables|/Script/Engine.Actor|GetRootComponent _array_element) false true)
        (Collision|SetActorEnableCollision _array_element false)))
    (:then_1
      (bind _outactors_2 (Actor|GetAllActorswithTag (Variables|Default|GetOverworld)))
      (bind _output_get_2 (Variables|Default|SetOverworldActors _outactors_2))
      (for _array_element_2 _output_get_2
        (Rendering|SetVisibility (Variables|/Script/Engine.Actor|GetRootComponent _array_element_2) true true)
        (Collision|SetActorEnableCollision _array_element_2 true)))
    (:then_2
      (bind _outactors_3 (Actor|GetAllActorsOfClass "/Game/Blueprints/Portal_BP.Portal_BP_C"))
      (EventDispatchers|BindEventtoPortalEntered (Utilities|Array|Get(acopy) _outactors_3) (delegate Custom|PortalEntered_Event)))))

(fn ConstructionScript)